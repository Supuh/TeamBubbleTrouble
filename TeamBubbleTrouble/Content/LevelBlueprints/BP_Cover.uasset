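; BP_Cover is an actor that endlessly slides its Plane component between two positions, apparently as moving cover.
; A self-calling MoveCover event, started at BeginPlay, waits, eases the plane to CoverEndLoc over a set travel time, pauses, then sends it back.
; The return move uses the default target and duration; the saved StartingLoc is never used.
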(event Custom|MoveCover
  (Utilities|FlowControl|Delay (Variables|Default|GetDelayUntilMove))
  (Components|MoveComponentTo (Variables|Default|GetPlane) (Variables|Default|GetCoverEndLoc) "0, 0, 0" false true (Variables|Default|GetTimeToTravel) false)
  (Utilities|FlowControl|Delay (Variables|Default|GetTimeToReset))
  (Development|PrintString "Return")
  (Components|MoveComponentTo (Variables|Default|GetPlane) "0, 0, 0" "0, 0, 0" false true 0.2 false)
  (CallFunction|MoveCover))

(event EventBeginPlay
  (Variables|Default|SetStartingLoc (Transformation|GetWorldLocation (Variables|Default|GetPlane)))
  (CallFunction|MoveCover))

(event Collision|EventActorBeginOverlap
  (params (OtherActor :type Actor%20Object%20Reference)))

(event EventTick
  (params (DeltaSeconds :type Float%20%28single-precision%29)))

(fn ConstructionScript)