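; BP_Bread is a jump pad actor that boosts the jump height of BP_ThirdPersonCharacterDavid while it stands inside the pad's box.
; Box overlap sets an OnBread flag and multiplies the character's JumpZVelocity by JumpMultiplier, then resets it to a hard-coded default on exit.
; Space bar or IA_Jump plays an explosion sound at the cube while OnBread is set, alongside debug prints.
; The construction script sizes the box from BoxVolume.
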(event OnComponentBeginOverlap(Box)
  (params (OverlappedComponent :type Primitive%20Component%20Object%20Reference) (OtherActor :type Actor%20Object%20Reference) (OtherComp :type Primitive%20Component%20Object%20Reference) (OtherBodyIndex :type Integer) (bFromSweep :type Boolean) (SweepResult :type Hit%20Result%20Structure%20%28by%20ref%29))
  (Variables|Default|SetOnBread? true)
  (bind _asbp_third_person_character_david (Utilities|Casting|CastToBP_ThirdPersonCharacterDavid OtherActor))
  (Variables|/Script/Engine.CharacterMovementComponent|SetJumpZVelocity (Variables|/Script/Engine.Character|GetCharacterMovement _asbp_third_person_character_david) (* (Variables|/Script/Engine.CharacterMovementComponent|GetJumpZVelocity (Variables|/Script/Engine.Character|GetCharacterMovement _asbp_third_person_character_david)) (Variables|Default|GetJumpMultiplier))))

(event OnComponentEndOverlap(Box)
  (params (OverlappedComponent :type Primitive%20Component%20Object%20Reference) (OtherActor :type Actor%20Object%20Reference) (OtherComp :type Primitive%20Component%20Object%20Reference) (OtherBodyIndex :type Integer))
  (Variables|Default|SetOnBread? false)
  (bind _asbp_third_person_character_david (Utilities|Casting|CastToBP_ThirdPersonCharacterDavid OtherActor))
  (Variables|/Script/Engine.CharacterMovementComponent|SetJumpZVelocity (Variables|/Script/Engine.Character|GetCharacterMovement _asbp_third_person_character_david) 7e+02))

(event Input|EnhancedActionEvents|EnhancedInputActionIA_Jump
  (params (ActionValue :type Boolean) (ElapsedSeconds :type Float%20%28double-precision%29) (TriggeredSeconds :type Float%20%28double-precision%29) (InputAction :type Input%20Action%20Object%20Reference :default "/Game/ThirdPerson/Input/Actions/IA_Jump.IA_Jump"))
  (bind _onbread_ (Variables|Default|GetOnBread?))
  (Development|PrintString (Utilities|String|ToString(Boolean) _onbread_))
  (if _onbread_
    (Audio|PlaySoundatLocation "/Game/StarterContent/Audio/Explosion01.Explosion01" (Transformation|GetWorldLocation (Variables|Default|GetCube)) "0, 0, 0" 1.0 1.0 0.0 0 0 0 0)
    (Development|PrintString "Hello")))

(event EventBeginPlay)

(event Collision|EventActorBeginOverlap
  (params (OtherActor :type Actor%20Object%20Reference)))

(event EventTick
  (params (DeltaSeconds :type Float%20%28single-precision%29)))

(event Input|KeyboardEvents|SpaceBar
  (params (Key :type Key%20Structure :default "None"))
  (bind _onbread_ (Variables|Default|GetOnBread?))
  (:Pressed
    (Development|PrintString (Utilities|String|ToString(Boolean) _onbread_))
    (if _onbread_
      (Audio|PlaySoundatLocation "/Game/StarterContent/Audio/Explosion01.Explosion01" (Transformation|GetWorldLocation (Variables|Default|GetCube)) "0, 0, 0" 1.0 1.0 0.0 0 0 0 0)
      (Development|PrintString "Hello"))))

(fn ConstructionScript
  (Components|Box|SetBoxExtent (Variables|Default|GetBox) (Variables|Default|GetBox%20Volume) true))