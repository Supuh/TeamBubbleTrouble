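; BP_Fruit is a rolling fruit hazard that launches itself forward and knocks the player character away.
; From BeginPlay, PushFruit loops on a delay, enabling physics on the Sphere and applying a forward impulse.
; Hitting BP_ThirdPersonCharacterDavid pushes its movement outward from the sphere's center and plays a rolling sound.
; ResetPos, not called within this Blueprint, moves the sphere back to the root, swapping to an invisible material meanwhile, and disables physics.
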(event OnComponentHit(Sphere)
  (params (HitComponent :type Primitive%20Component%20Object%20Reference) (OtherActor :type Actor%20Object%20Reference) (OtherComp :type Primitive%20Component%20Object%20Reference) (NormalImpulse :type Vector :default "0, 0, 0") (Hit :type Hit%20Result%20Structure%20%28by%20ref%29))
  (bind _asbp_third_person_character_david (Utilities|Casting|CastToBP_ThirdPersonCharacterDavid OtherActor))
  (Physics|AddImpulse (Variables|/Script/Engine.Character|GetCharacterMovement _asbp_third_person_character_david) (* (- (.location Hit) (Transformation|GetWorldLocation (Variables|Default|GetSphere))) 1e+01) true)
  (Utilities|FlowControl|DoOnce false :!label _label
    (:Completed
      (Audio|PlaySoundatLocation "/Game/LevelBlueprints/FruitRolling.FruitRolling" (Transformation|GetWorldLocation (Variables|Default|GetSphere)) "0, 0, 0" 1.0 1.0 0.0 0 0 0 0)
      (goto _label Reset))))

(event Custom|PushFruit
  (Utilities|FlowControl|Delay (Variables|Default|GetStaticDuration))
  (Physics|SetSimulatePhysics (Variables|Default|GetSphere) true)
  (Physics|AddImpulse (Variables|Default|GetSphere) (* (Math|Vector|GetForwardVector (Variables|Default|GetSphere)) (Variables|Default|GetForceAmount)) "None" true)
  (CallFunction|PushFruit))

(event Custom|ResetPos
  (bind _defaultsceneroot (Variables|Default|GetDefaultSceneRoot))
  (bind _sphere (Variables|Default|GetSphere))
  (Rendering|Material|SetMaterial (Variables|Default|GetSphere) 0 "/Game/LevelBlueprints/M_Invisible.M_Invisible")
  (Components|MoveComponentTo _sphere (Transformation|GetWorldLocation _defaultsceneroot) (Transformation|GetWorldRotation _defaultsceneroot) false false 0.2 false)
  (Rendering|Material|SetMaterial (Variables|Default|GetSphere) 0 (Variables|Default|GetBaseMaterial))
  (Physics|SetSimulatePhysics (Variables|Default|GetSphere) false)
  (Development|PrintString (Utilities|String|ToString(Vector) (Transformation|GetWorldLocation _sphere))))

(event EventBeginPlay
  (Variables|Default|SetBaseMaterial (Rendering|Material|GetMaterial (Variables|Default|GetSphere) 0))
  (CallFunction|PushFruit))

(fn ConstructionScript)