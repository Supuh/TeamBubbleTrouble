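; BP_Jam is an area actor that alters BP_TestChar's walk speed inside a sphere sized by SphereRadius at construction.
; Entering multiplies MaxWalkSpeed by MoveSpeedModifier and plays a fire sound; leaving sets a hard-coded speed rather than restoring the previous one.
; BP_ThirdPersonCharacter overlap paths are disconnected, and the movement component cached on BeginPlay is unused.
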(event OnComponentBeginOverlap(Sphere1)
  (params (OverlappedComponent :type Primitive%20Component%20Object%20Reference) (OtherActor :type Actor%20Object%20Reference) (OtherComp :type Primitive%20Component%20Object%20Reference) (OtherBodyIndex :type Integer) (bFromSweep :type Boolean) (SweepResult :type Hit%20Result%20Structure%20%28by%20ref%29))
  (bind _asbp_test_char (Utilities|Casting|CastToBP_TestChar OtherActor))
  (Variables|/Script/Engine.CharacterMovementComponent|SetMaxWalkSpeed (Variables|/Script/Engine.Character|GetCharacterMovement _asbp_test_char) (* (Variables|/Script/Engine.CharacterMovementComponent|GetMaxWalkSpeed (Variables|/Script/Engine.Character|GetCharacterMovement _asbp_test_char)) (Variables|Default|GetMoveSpeedModifier)))
  (Audio|PlaySoundatLocation "/Game/StarterContent/Audio/Fire01.Fire01" (Transformation|GetWorldLocation (Variables|Default|GetSphere)) "0, 0, 0" 1.0 1.0 0.0 0 0 0 0)
  (Utilities|FlowControl|DoOnce false))

(event OnComponentEndOverlap(Sphere1)
  (params (OverlappedComponent :type Primitive%20Component%20Object%20Reference) (OtherActor :type Actor%20Object%20Reference) (OtherComp :type Primitive%20Component%20Object%20Reference) (OtherBodyIndex :type Integer))
  (bind _asbp_test_char (Utilities|Casting|CastToBP_TestChar OtherActor))
  (Variables|/Script/Engine.CharacterMovementComponent|SetMaxWalkSpeed (Variables|/Script/Engine.Character|GetCharacterMovement _asbp_test_char) 5e+02))

(event EventBeginPlay
  (bind _asbp_third_person_character (Utilities|Casting|CastToBP_ThirdPersonCharacter (Game|GetPlayerCharacter 0)))
  (Variables|Default|SetDefaultMovement (Variables|/Script/Engine.Character|GetCharacterMovement _asbp_third_person_character)))

(fn ConstructionScript
  (Components|Sphere|SetSphereRadius (Variables|Default|GetSphere1) (Variables|Default|GetSphere%20Radius) true))