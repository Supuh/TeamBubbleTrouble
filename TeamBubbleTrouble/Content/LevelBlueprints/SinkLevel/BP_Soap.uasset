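; BP_Soap is a soap actor for the sink level that leaves BP_SlippyZone actors where it hits surfaces.
; When its Cube component registers a hit, it spawns a zone at the impact point if it overlaps none.
; Otherwise it prints a debug string and spawns an active zone for each inactive zone it overlaps.
; Unconnected sphere trace, SlipChecker overlap and timer nodes never run.
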(event OnComponentHit(Cube)
  (params (HitComponent :type Primitive%20Component%20Object%20Reference) (OtherActor :type Actor%20Object%20Reference) (OtherComp :type Primitive%20Component%20Object%20Reference) (NormalImpulse :type Vector :default "0, 0, 0") (Hit :type Hit%20Result%20Structure%20%28by%20ref%29))
  (bind _overlappingactors (Collision|GetOverlappingActors "/Game/LevelBlueprints/SinkLevel/BP_SlippyZone.BP_SlippyZone_C" :!class /Script/Engine.Actor))
  (bind _returnvalue (Utilities|Array|IsEmpty _overlappingactors))
  (bind _output_get (Variables|Default|SetHit Hit))
  (if _returnvalue
    (Game|SpawnActorfromClass "/Game/LevelBlueprints/SinkLevel/BP_SlippyZone.BP_SlippyZone_C" (Math|Transform|MakeTransform (.location _output_get) "0, 0, 0" "1.000000,1.000000,1.000000") "AdjustIfPossibleButDontSpawnIfColliding" "MultiplyWithRoot" 0 0)
    (else
      (Development|PrintString (Utilities|String|ToString(Boolean) _returnvalue))
      (for _array_element _overlappingactors
        (if (not (Variables|/Game/LevelBlueprints/SinkLevel/BP_SlippyZone.BP_SlippyZone_C|GetisActive? _array_element))
          (bind _returnvalue_2 (Game|SpawnActorfromClass "/Game/LevelBlueprints/SinkLevel/BP_SlippyZone.BP_SlippyZone_C" (Math|Transform|MakeTransform (.location _output_get) "0, 0, 0" "1.000000,1.000000,1.000000") "AdjustIfPossibleButDontSpawnIfColliding" "MultiplyWithRoot" 0 0))
          (Variables|/Game/LevelBlueprints/SinkLevel/BP_SlippyZone.BP_SlippyZone_C|SetisActive? _returnvalue_2 true))))))

(fn ConstructionScript)