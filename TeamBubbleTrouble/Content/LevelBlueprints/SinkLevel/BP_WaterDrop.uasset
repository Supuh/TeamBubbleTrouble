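; BP_WaterDrop is a water drop hazard in the sink level that splashes on impact and pushes the test character.
; On a sphere hit, it enlarges the collision radius by a multiplier, waits a second, then destroys itself.
; A BP_TestChar that begins overlapping the sphere receives a movement impulse along its mesh's forward vector, scaled by PushbackMultiplier.
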(event OnComponentHit(Sphere)
  (params (HitComponent :type Primitive%20Component%20Object%20Reference) (OtherActor :type Actor%20Object%20Reference) (OtherComp :type Primitive%20Component%20Object%20Reference) (NormalImpulse :type Vector :default "0, 0, 0") (Hit :type Hit%20Result%20Structure%20%28by%20ref%29))
  (Variables|Default|SetHit Hit)
  (Components|Sphere|SetSphereRadius (Variables|Default|GetSphere) (* (Variables|Default|GetBase%20Radus) (Variables|Default|GetBigDropRadius)) true)
  (Utilities|FlowControl|Delay 1.0)
  (Actor|DestroyActor))

(event OnComponentBeginOverlap(Sphere)
  (params (OverlappedComponent :type Primitive%20Component%20Object%20Reference) (OtherActor :type Actor%20Object%20Reference) (OtherComp :type Primitive%20Component%20Object%20Reference) (OtherBodyIndex :type Integer) (bFromSweep :type Boolean) (SweepResult :type Hit%20Result%20Structure%20%28by%20ref%29))
  (bind _asbp_test_char (Utilities|Casting|CastToBP_TestChar OtherActor))
  (Physics|AddImpulse (Variables|/Script/Engine.Character|GetCharacterMovement _asbp_test_char) (* (Math|Vector|GetForwardVector (Variables|/Script/Engine.Character|GetMesh _asbp_test_char)) (Variables|Default|GetPushback%20multiplier)) false))

(event EventBeginPlay
  (Variables|Default|SetBase%20Radus (Variables|/Script/Engine.SphereComponent|GetSphereRadius (Variables|Default|GetSphere))))

(event Collision|EventActorBeginOverlap
  (params (OtherActor :type Actor%20Object%20Reference)))

(event EventTick
  (params (DeltaSeconds :type Float%20%28single-precision%29)))

(fn ConstructionScript)