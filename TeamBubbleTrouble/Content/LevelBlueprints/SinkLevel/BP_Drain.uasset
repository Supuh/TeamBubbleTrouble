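; BP_Drain is a sink-level drain hazard that sucks the player character toward its center.
; Entering its sphere, whose radius is set in the construction script, sets an in-area flag and starts a looping timer.
; While flagged, each tick of that timer applies a PullStrength-scaled impulse toward the sphere and prints it for debugging.
; Exiting clears the flag without stopping the timer; alternative movement approaches remain unconnected.
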(event OnComponentBeginOverlap(Sphere)
  (params (OverlappedComponent :type Primitive%20Component%20Object%20Reference) (OtherActor :type Actor%20Object%20Reference) (OtherComp :type Primitive%20Component%20Object%20Reference) (OtherBodyIndex :type Integer) (bFromSweep :type Boolean) (SweepResult :type Hit%20Result%20Structure%20%28by%20ref%29))
  (Variables|Default|SetInArea? true)
  (Utilities|Time|SetTimerbyEvent (delegate Custom|ApplyDrainForce) 0.1 true))

(event OnComponentEndOverlap(Sphere)
  (params (OverlappedComponent :type Primitive%20Component%20Object%20Reference) (OtherActor :type Actor%20Object%20Reference) (OtherComp :type Primitive%20Component%20Object%20Reference) (OtherBodyIndex :type Integer))
  (Variables|Default|SetInArea? false)
  (Development|PrintString "Exited Drain"))

(event Custom|ApplyDrainForce
  (bind _sphere (Variables|Default|GetSphere))
  (bind _as_bp_third_person_character (Variables|Default|GetAs%20BP%20Third%20Person%20Character))
  (bind _pullstrength (Variables|Default|GetPullStrength))
  (bind _returnvalue (Transformation|GetWorldLocation _sphere))
  (bind _capsulecomponent (Variables|/Script/Engine.Character|GetCapsuleComponent _as_bp_third_person_character))
  (bind _returnvalue_2 (Transformation|GetWorldLocation _capsulecomponent))
  (bind _returnvalue_3 (- _returnvalue _returnvalue_2))
  (bind _returnvalue_4 (Math|Vector|Normalize _returnvalue_3))
  (bind _returnvalue_5 (* _returnvalue_4 (Math|Vector|MakeVector _pullstrength _pullstrength _pullstrength)))
  (if (Variables|Default|GetInArea?)
    (Physics|AddImpulse (Variables|/Script/Engine.Character|GetCharacterMovement (Variables|Default|GetAs%20BP%20Third%20Person%20Character)) _returnvalue_5 false)
    (Development|PrintString (Utilities|String|ToString(Vector) _returnvalue_5))))

(event EventBeginPlay
  (bind _asbp_third_person_character (Utilities|Casting|CastToBP_ThirdPersonCharacter (Game|GetPlayerCharacter 0)))
  (Variables|Default|SetAs%20BP%20Third%20Person%20Character _asbp_third_person_character))

(fn ConstructionScript
  (Components|Sphere|SetSphereRadius (Variables|Default|GetSphere) (Variables|Default|GetRadius) true))