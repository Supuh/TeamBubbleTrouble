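; Water drip hazard for the sink level that pushes the third-person character when it touches the drip.
; On BeginPlay it sets the capsule radius, then a timeline drives the capsule half-height scaled by drip length, replaying after a delay each cycle.
; Capsule overlap applies an impulse to the character along its mesh forward vector, scaled by a pushback multiplier.
; Several leftover node chains are unconnected and never run.
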(event OnComponentBeginOverlap(Capsule)
  (params (OverlappedComponent :type Primitive%20Component%20Object%20Reference) (OtherActor :type Actor%20Object%20Reference) (OtherComp :type Primitive%20Component%20Object%20Reference) (OtherBodyIndex :type Integer) (bFromSweep :type Boolean) (SweepResult :type Hit%20Result%20Structure%20%28by%20ref%29))
  (bind _asbp_third_person_character (Utilities|Casting|CastToBP_ThirdPersonCharacter OtherActor))
  (Physics|AddImpulse (Variables|/Script/Engine.Character|GetCharacterMovement _asbp_third_person_character) (* (Math|Vector|GetForwardVector (Variables|/Script/Engine.Character|GetMesh _asbp_third_person_character)) (Variables|Default|GetPushback%20multiplier)) false))

(event EventBeginPlay
  (Components|Capsule|SetCapsuleRadius (Variables|Default|GetCapsule) (Variables|Default|GetRadius) true)
  (Components|Timeline|SetPlayRate (Variables|Default|GetTimeline) 1.0)
  (bind _driplength (Timeline|Timeline Play)
    (:Update
      (Components|Capsule|SetCapsuleHalfHeight (Variables|Default|GetCapsule) (* _driplength (Variables|Default|GetDripLength)) true))
    (:Finished
      (Utilities|FlowControl|Delay (Variables|Default|GetDelay%20Duration))
      (Timeline|Timeline PlayFromStart))))

(event Collision|EventActorBeginOverlap
  (params (OtherActor :type Actor%20Object%20Reference)))

(event EventTick
  (params (DeltaSeconds :type Float%20%28single-precision%29)))

(fn ConstructionScript)