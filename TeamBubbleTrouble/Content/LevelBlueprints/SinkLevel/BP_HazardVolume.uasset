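; BP_HazardVolume is a damage zone whose box extent is set from BoxVolume in the construction script.
; Overlap begin clears Exited and starts DamageHealth, which damages the actor, lowers and prints a DummyHealth counter, then re-calls itself every second until overlap end sets Exited.
; The repeat call passes no actor, so only the first ApplyDamage receives the overlapping actor.
; BeginPlay caches the player character, which is otherwise unused.
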(event OnComponentBeginOverlap(Box)
  (params (OverlappedComponent :type Primitive%20Component%20Object%20Reference) (OtherActor :type Actor%20Object%20Reference) (OtherComp :type Primitive%20Component%20Object%20Reference) (OtherBodyIndex :type Integer) (bFromSweep :type Boolean) (SweepResult :type Hit%20Result%20Structure%20%28by%20ref%29))
  (Variables|Default|SetExited? false)
  (CallFunction|DamageHealth OtherActor))

(event OnComponentEndOverlap(Box)
  (params (OverlappedComponent :type Primitive%20Component%20Object%20Reference) (OtherActor :type Actor%20Object%20Reference) (OtherComp :type Primitive%20Component%20Object%20Reference) (OtherBodyIndex :type Integer))
  (Variables|Default|SetExited? true))

(event Custom|DamageHealth
  (params (DamagedActor :type Actor%20Object%20Reference))
  (if (not (Variables|Default|GetExited?))
    (Game|Damage|ApplyDamage DamagedActor (Variables|Default|GetDamage%20amount) 0 0)
    (bind _output_get (Variables|Default|SetDummyHealth (- (Variables|Default|GetDummyHealth) (Variables|Default|GetDamage%20amount))))
    (Development|PrintString (Utilities|String|ToString(Float) _output_get))
    (Utilities|FlowControl|Delay 1.0)
    (CallFunction|DamageHealth)))

(event EventBeginPlay
  (bind _asbp_third_person_character (Utilities|Casting|CastToBP_ThirdPersonCharacter (Game|GetPlayerCharacter 0)))
  (Variables|Default|SetAs%20BP%20Third%20Person%20Character _asbp_third_person_character))

(fn ConstructionScript
  (Components|Box|SetBoxExtent (Variables|Default|GetBox) (Variables|Default|GetBox%20Volume) true))