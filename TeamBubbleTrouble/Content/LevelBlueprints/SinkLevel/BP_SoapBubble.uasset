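; BP_SoapBubble is a sink-level soap bubble that pushes the player away on contact.
; An overlap on Sphere1 plays a sound at the Sphere component for any actor, then casts to BP_ThirdPersonCharacterDavid.
; That character receives a velocity-change impulse along the vector from Sphere to its capsule, scaled by PushBackForce and not normalized.
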(event OnComponentBeginOverlap(Sphere1)
  (params (OverlappedComponent :type Primitive%20Component%20Object%20Reference) (OtherActor :type Actor%20Object%20Reference) (OtherComp :type Primitive%20Component%20Object%20Reference) (OtherBodyIndex :type Integer) (bFromSweep :type Boolean) (SweepResult :type Hit%20Result%20Structure%20%28by%20ref%29))
  (Audio|PlaySoundatLocation "/Game/LevelBlueprints/SinkLevel/by_chance.by_chance" (Transformation|GetWorldLocation (Variables|Default|GetSphere)) "0, 0, 0" 1.0 1.0 0.0 0 0 0 0)
  (bind _asbp_third_person_character_david (Utilities|Casting|CastToBP_ThirdPersonCharacterDavid OtherActor))
  (Physics|AddImpulse (Variables|/Script/Engine.Character|GetCharacterMovement _asbp_third_person_character_david) (* (- (Transformation|GetWorldLocation (Variables|/Script/Engine.Character|GetCapsuleComponent _asbp_third_person_character_david)) (Transformation|GetWorldLocation (Variables|Default|GetSphere))) (Variables|Default|GetPushBackForce)) true))

(event EventBeginPlay)

(event Collision|EventActorBeginOverlap
  (params (OtherActor :type Actor%20Object%20Reference)))

(event EventTick
  (params (DeltaSeconds :type Float%20%28single-precision%29)))

(fn ConstructionScript)