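; BP_Faucet is a faucet actor for the Sink level that emits a water drip.
; On BeginPlay it spawns a BP_WaterDrip at its Arrow component's world transform, passing along its DripLength and Radius values.
; Unconnected leftover nodes for playing ShotPatterns and spawning BP_WaterDrop never run, and the construction script is empty.
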(event EventBeginPlay
  (Game|SpawnActorfromClass "/Game/LevelBlueprints/SinkLevel/BP_WaterDrip.BP_WaterDrip_C" (Transformation|GetWorldTransform (Variables|Default|GetArrow)) "Undefined" "MultiplyWithRoot" 0 (Variables|Default|GetDrip%20Length) (Variables|Default|GetRadius) 1.0 0))

(event Collision|EventActorBeginOverlap
  (params (OtherActor :type Actor%20Object%20Reference)))

(event EventTick
  (params (DeltaSeconds :type Float%20%28single-precision%29)))

(fn ConstructionScript)