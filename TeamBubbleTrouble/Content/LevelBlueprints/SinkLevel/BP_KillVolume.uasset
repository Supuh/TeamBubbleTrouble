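; BP_KillVolume is a box volume in the SinkLevel folder, apparently an unfinished hazard meant to damage actors inside it.
; The construction script sizes the box from BoxVolume.
; DamageHealth applies damage, lowers and prints a DummyHealth counter, then repeats each second until Exited is set.
; Nothing live starts that loop: begin overlap only casts to BP_TestChar, end overlap is empty, and the trigger logic is disconnected.
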(event OnComponentBeginOverlap(Box)
  (params (OverlappedComponent :type Primitive%20Component%20Object%20Reference) (OtherActor :type Actor%20Object%20Reference) (OtherComp :type Primitive%20Component%20Object%20Reference) (OtherBodyIndex :type Integer) (bFromSweep :type Boolean) (SweepResult :type Hit%20Result%20Structure%20%28by%20ref%29))
  (Utilities|Casting|CastToBP_TestChar OtherActor))

(event OnComponentEndOverlap(Box)
  (params (OverlappedComponent :type Primitive%20Component%20Object%20Reference) (OtherActor :type Actor%20Object%20Reference) (OtherComp :type Primitive%20Component%20Object%20Reference) (OtherBodyIndex :type Integer)))

(event Custom|DamageHealth
  (params (DamagedActor :type Actor%20Object%20Reference))
  (if (not (Variables|Default|GetExited?))
    (Game|Damage|ApplyDamage DamagedActor (Variables|Default|GetDamage%20amount) 0 0)
    (bind _output_get (Variables|Default|SetDummyHealth (- (Variables|Default|GetDummyHealth) (Variables|Default|GetDamage%20amount))))
    (Development|PrintString (Utilities|String|ToString(Float) _output_get))
    (Utilities|FlowControl|Delay 1.0)
    (CallFunction|DamageHealth)))

(event EventBeginPlay)

(fn ConstructionScript
  (Components|Box|SetBoxExtent (Variables|Default|GetBox) (Variables|Default|GetBox%20Volume) true))