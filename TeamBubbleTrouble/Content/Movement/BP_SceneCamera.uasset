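; BP_SceneCamera is a shared camera actor that frames two BP_ThirdPersonCharacterDavid players at once.
; Shortly after BeginPlay it becomes player 0's view target, caches all those characters and enables ticking.
; Each tick it moves to the midpoint of the first two and scales spring arm length with their distance, clamped to keep zoom within bounds.
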(event EventBeginPlay
  (Utilities|FlowControl|Delay 0.01)
  (Game|Player|SetViewTargetwithBlend (Game|GetPlayerController 0) self 0.0 "VTBlend_Linear" 0.0 false)
  (bind _outactors (Actor|GetAllActorsOfClass "/Game/David/BP_ThirdPersonCharacterDavid.BP_ThirdPersonCharacterDavid_C"))
  (Variables|Default|SetPlayers _outactors)
  (Actor|Tick|SetActorTickEnabled true))

(event EventTick
  (params (DeltaSeconds :type Float%20%28single-precision%29))
  (bind _players (Variables|Default|GetPlayers))
  (bind _output (Utilities|Array|Get(acopy) _players 1))
  (bind _output_2 (Utilities|Array|Get(acopy) _players))
  (Variables|/Script/Engine.SpringArmComponent|SetTargetArmLength (Variables|Default|GetSpringArm) (Math|Float|Clamp(Float) (* (Transformation|GetDistanceTo _output_2 _output) 2.0) 4e+02 1.5e+03))
  (Transformation|SetActorLocation (Math|Vector|Lerp(Vector) (Transformation|GetActorLocation _output_2) (Transformation|GetActorLocation _output) 0.5) false false))

(fn ConstructionScript)