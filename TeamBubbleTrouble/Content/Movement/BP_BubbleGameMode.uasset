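; Game mode Blueprint whose live logic is empty: BeginPlay and the construction script do nothing.
; Disconnected draft graphs sketch local multiplayer, creating a player per PlayerStart, adding the default Enhanced Input context and possessing a spawned BP_TestChar.
; Their additional-player branch tests 0 > index, so every start would fall through to the Player 1 path.
; A second unwired loop just creates extra local players.
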(event EventBeginPlay)

(fn ConstructionScript)